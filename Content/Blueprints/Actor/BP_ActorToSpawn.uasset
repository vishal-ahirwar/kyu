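; BP_ActorToSpawn is a spawnable level segment with trigger volumes that react only to the player pawn, apparently for an endless-runner style loop.
; Entering Box calls SpawnBase on BP_kyuGameModeBase and adds to its Score, while leaving Box1 gives the segment a short lifespan for cleanup.
; Touching Box2 or W destroys the player and immediately reloads the current level, as the Delay nodes are left disconnected.
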(event `self.Box.OnComponentBeginOverlap`
  (params (OverlappedComponent :type "PrimitiveComponent Object Reference") (OtherActor :type "Actor Object Reference") (OtherComp :type "PrimitiveComponent Object Reference") (OtherBodyIndex :type Integer) (bFromSweep :type Boolean) (SweepResult :type "HitResult Structure (by ref)"))
  (if (== OtherActor (`GameplayStatics.GetPlayerPawn` 0))
    (bind _asbp_kyu_game_mode_base (cast `/Game/Blueprints/GameMode/BP_kyuGameModeBase` (`GameplayStatics.GetGameMode`)))
    (`/Game/Blueprints/GameMode/BP_kyuGameModeBase.SpawnBase` _asbp_kyu_game_mode_base)
    (set `/Game/Blueprints/GameMode/BP_kyuGameModeBase.Score` (+ (`/Game/Blueprints/GameMode/BP_kyuGameModeBase.Score` _asbp_kyu_game_mode_base) 5) _asbp_kyu_game_mode_base)))

(event `self.Box1.OnComponentEndOverlap`
  (params (OverlappedComponent :type "PrimitiveComponent Object Reference") (OtherActor :type "Actor Object Reference") (OtherComp :type "PrimitiveComponent Object Reference") (OtherBodyIndex :type Integer))
  (if (== OtherActor (`GameplayStatics.GetPlayerPawn` 0))
    (`self.SetLifeSpan` 3.0)))

(event `self.Box2.OnComponentBeginOverlap`
  (params (OverlappedComponent :type "PrimitiveComponent Object Reference") (OtherActor :type "Actor Object Reference") (OtherComp :type "PrimitiveComponent Object Reference") (OtherBodyIndex :type Integer) (bFromSweep :type Boolean) (SweepResult :type "HitResult Structure (by ref)"))
  (bind _returnvalue (`GameplayStatics.GetPlayerPawn` 0))
  (if (== OtherActor _returnvalue)
    (`self.K2_DestroyActor` _returnvalue)
    (bind _returnvalue_2 (`GameplayStatics.GetCurrentLevelName` true))
    (`GameplayStatics.OpenLevel` (`KismetStringLibrary.Conv_StringToName` _returnvalue_2))))

(event `self.w.OnComponentBeginOverlap`
  (params (OverlappedComponent :type "PrimitiveComponent Object Reference") (OtherActor :type "Actor Object Reference") (OtherComp :type "PrimitiveComponent Object Reference") (OtherBodyIndex :type Integer) (bFromSweep :type Boolean) (SweepResult :type "HitResult Structure (by ref)"))
  (bind _returnvalue (`GameplayStatics.GetPlayerPawn` 0))
  (if (== OtherActor _returnvalue)
    (`self.K2_DestroyActor` _returnvalue)
    (bind _returnvalue_2 (`GameplayStatics.GetCurrentLevelName` true))
    (`GameplayStatics.OpenLevel` (`KismetStringLibrary.Conv_StringToName` _returnvalue_2))))

(fn `UserConstructionScript`)