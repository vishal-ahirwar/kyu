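; Base player pawn that restarts the current level on collision and opens the pause menu.
; Any hit on the Root component immediately reopens the level by name; an unused destroy-and-delay branch is left disconnected.
; The Pause input reveals a box in the widget held by BP_kyuGameModeBase, pauses the game, switches to UI-only input and shows the mouse cursor.
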(event `self.Root.OnComponentHit`
  (params (HitComponent :type "PrimitiveComponent Object Reference") (OtherActor :type "Actor Object Reference") (OtherComp :type "PrimitiveComponent Object Reference") (NormalImpulse :type "Vector Structure") (Hit :type "HitResult Structure (by ref)"))
  (bind _returnvalue (`GameplayStatics.GetCurrentLevelName` true))
  (`GameplayStatics.OpenLevel` (`KismetStringLibrary.Conv_StringToName` _returnvalue)))

(event `InputAction|Pause`
  (params (Key :type "Key Structure"))
  (bind _returnvalue (`GameplayStatics.GetPlayerController` 0))
  (:`Pressed`
    (bind _asbp_kyu_game_mode_base (cast `/Game/Blueprints/GameMode/BP_kyuGameModeBase` (`GameplayStatics.GetGameMode`)))
    (`Widget.SetVisibility` (`/Game/Widgets/WBP_GameMenu.VerticalBox_0` (`/Game/Blueprints/GameMode/BP_kyuGameModeBase.Widget` _asbp_kyu_game_mode_base)) "Visible")
    (`GameplayStatics.SetGamePaused` true)
    (`WidgetBlueprintLibrary.SetInputMode_UIOnlyEx` _returnvalue null)
    (set `PlayerController.bShowMouseCursor` true _returnvalue)))

(fn `UserConstructionScript`)