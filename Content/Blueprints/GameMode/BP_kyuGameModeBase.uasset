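; Game mode that creates the game menu widget and builds a randomly assembled chain of actors when play begins.
; BeginPlay adds the menu to the viewport, then calls SpawnBase in a fixed-count loop.
; SpawnBase picks one of three actor classes at random, spawns it at NextSpawnLocation, then moves that location to the new actor's SpawnPoint, linking each piece to the previous one.
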(event `self.ReceiveBeginPlay`
  (bind _returnvalue (`|CreateWidget` "/Game/Widgets/WBP_GameMenu.WBP_GameMenu_C"))
  (set `self.Widget` _returnvalue)
  (`UserWidget.AddToViewport` _returnvalue 0)
  (for _ (range 11)
    (`self.SpawnBase`)))

(fn `SpawnBase`
  (switch `int` (`KismetMathLibrary.RandomIntegerInRange` 0 2)
    (:`0`
      (bind _returnvalue (`|SpawnActorFromClass` "/Game/Blueprints/Actor/BP_ActorToSpawn.BP_ActorToSpawn_C" (`KismetMathLibrary.MakeTransform` (`self.NextSpawnLocation`)) "Undefined" "OverrideRootScale" null null))
      (set `self.NextSpawnLocation` (`SceneComponent.K2_GetComponentLocation` (`/Game/Blueprints/Actor/BP_ActorToSpawn.Spawn Point` _returnvalue))))
    (:`1`
      (bind _returnvalue_2 (`|SpawnActorFromClass` "/Game/Blueprints/Actor/BP_ActorToSpawn1.BP_ActorToSpawn1_C" (`KismetMathLibrary.MakeTransform` (`self.NextSpawnLocation`)) "Undefined" "OverrideRootScale" null null))
      (set `self.NextSpawnLocation` (`SceneComponent.K2_GetComponentLocation` (`/Game/Blueprints/Actor/BP_ActorToSpawn1.Spawn Point` _returnvalue_2))))
    (:`2`
      (bind _returnvalue_3 (`|SpawnActorFromClass` "/Game/Blueprints/Actor/BP_ActorToSpawn2.BP_ActorToSpawn2_C" (`KismetMathLibrary.MakeTransform` (`self.NextSpawnLocation`)) "Undefined" "OverrideRootScale" null null))
      (set `self.NextSpawnLocation` (`SceneComponent.K2_GetComponentLocation` (`/Game/Blueprints/Actor/BP_ActorToSpawn2.Spawn Point` _returnvalue_3))))))

(fn `UserConstructionScript`)